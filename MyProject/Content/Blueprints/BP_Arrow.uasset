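; BP_Arrow is an arrow actor that rotates to point at the active stop (BP_Parada).
; On BeginPlay it scans all BP_Parada actors and caches the last one flagged BoolActive as CurrentActiveStop.
; Each Tick, while that reference is valid, it sets its rotation with FindLookAtRotation toward the stop.
; The target is chosen only at BeginPlay; nothing in this Blueprint updates it afterward.
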(event EventBeginPlay
  (bind _outactors (Actor|GetAllActorsOfClass "/Game/Blueprints/BP_Parada.BP_Parada_C"))
  (for _array_element _outactors
    (if (Variables|/Game/Blueprints/BP_Parada.BP_Parada_C|GetBool_Active _array_element)
      (Variables|Default|SetCurrentActiveStop _array_element))))

(event Collision|EventActorBeginOverlap
  (params (OtherActor :type Actor%20Object%20Reference)))

(event EventTick
  (params (DeltaSeconds :type Float%20%28single-precision%29))
  (if (Utilities|IsValid (Variables|Default|GetCurrentActiveStop))
    (Transformation|SetActorRotation (Math|Rotator|FindLookatRotation (Transformation|GetActorLocation) (Transformation|GetActorLocation (Variables|Default|GetCurrentActiveStop))))))

(fn ConstructionScript)