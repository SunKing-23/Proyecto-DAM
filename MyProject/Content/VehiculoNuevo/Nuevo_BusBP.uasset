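; Drivable bus Blueprint that moves a physics box with custom raycast suspension, using Enhanced Input for throttle and steering.
; Each tick, four wheel traces apply compression-based spring forces, and grounded wheels also push forward by the Acceleration value, which input and CalculateAccel both write.
; Steering applies yaw torque to the box, and camera FOV widens with speed.
; It also attaches a BP_Arrow overhead and can display a passenger widget.
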(event Custom|ShowPassengerInterface
  (bind _returnvalue (UserInterface|CreateWidget "/Game/User_Interface/WBP_PassengerView.WBP_PassengerView_C" (Game|GetPlayerController 0)))
  (Variables|Default|SetPassengerWidget _returnvalue)
  (UserInterface|Viewport|AddtoViewport (Variables|Default|GetPassengerWidget) 0))

(event Input|EnhancedActionEvents|EnhancedInputActionAccelerate
  (params (ActionValue :type Float%20%28double-precision%29) (ElapsedSeconds :type Float%20%28double-precision%29) (TriggeredSeconds :type Float%20%28double-precision%29) (InputAction :type Input%20Action%20Object%20Reference :default "/Game/VehiculoNuevo/Inputs/Accelerate.Accelerate"))
  (Variables|Default|Setacceleration (Math|Interpolation|FInterpTo (Variables|Default|Getacceleration) ActionValue (Utilities|Time|GetWorldDeltaSeconds) 0.5)))

(event Input|EnhancedActionEvents|EnhancedInputActionSteer
  (params (ActionValue :type Float%20%28double-precision%29) (ElapsedSeconds :type Float%20%28double-precision%29) (TriggeredSeconds :type Float%20%28double-precision%29) (InputAction :type Input%20Action%20Object%20Reference :default "/Game/VehiculoNuevo/Inputs/Steer.Steer"))
  (Class|PrimitiveComponent|AddTorqueinRadians (Variables|Default|GetBox) (Math|Vector|MakeVector 0.0 0.0 (* ActionValue 8e+07)) "None" false))

(event EventBeginPlay
  (bind _returnvalue (Game|SpawnActorfromClass "/Game/Blueprints/BP_Arrow.BP_Arrow_C" (Math|Transform|MakeTransform "0, 0, 0" "0, 0, 0" "1.000000,1.000000,1.000000") "Undefined" "MultiplyWithRoot" 0 0))
  (Transformation|AttachComponentToComponent _returnvalue (Variables|Transformation|GetRootComponent) "None" "KeepRelative" "KeepRelative" "KeepRelative" true)
  (Transformation|SetRelativeLocation (Variables|/Script/Engine.Actor|GetRootComponent _returnvalue) "0.000000,0.000000,200.000000" false false)
  (Input|AddMappingContext (PlayerController|LocalPlayerSubsystems|GetEnhancedInputLocalPlayerSubsystem (Game|GetPlayerController 0)) "/Game/VehiculoNuevo/Inputs/Vehicle.Vehicle" 0 "(bIgnoreAllPressedKeysUntilRelease=True,bForceImmediately=False,bNotifyUserSettings=False)"))

(event Collision|EventActorBeginOverlap
  (params (OtherActor :type Actor%20Object%20Reference)))

(event EventTick
  (params (DeltaSeconds :type Float%20%28single-precision%29))
  (CallFunction|SuspensionCast (Variables|Default|GetFL_Wheel))
  (CallFunction|SuspensionCast (Variables|Default|GetFR_Wheel))
  (CallFunction|SuspensionCast (Variables|Default|GetBL_Wheel))
  (CallFunction|SuspensionCast (Variables|Default|GetBR_Wheel))
  (CallFunction|CalculateAccel)
  (CallFunction|FOVDinamico))

(fn ConstructionScript)

(fn SuspensionCast
  (params (WheelComp :type Scene%20Component%20Object%20Reference))
  (bind _returnvalue (Transformation|GetWorldLocation WheelComp))
  (bind _outhit (Collision|LineTraceByChannel _returnvalue (+ _returnvalue (* (Math|Vector|GetUpVector WheelComp) -6e+01)) "TraceTypeQuery1" false 0 "ForOneFrame"))
  (if (.bBlockingHit (Collision|BreakHitResult _outhit))
    (Class|PrimitiveComponent|AddForceatLocation (Variables|Default|GetBox) (* (- 1.0 (Math|Float|NormalizetoRange (.Distance (Collision|BreakHitResult _outhit)) 0.0 6e+01)) (Math|Vector|GetUnitDirection(Vector) (.TraceEnd (Collision|BreakHitResult _outhit)) (.TraceStart (Collision|BreakHitResult _outhit))) 2e+05) (Transformation|GetWorldLocation WheelComp) "None")
    (CallFunction|Accelerate WheelComp)))

(fn CalculateAccel
  (Variables|Default|Setacceleration (* (Math|Float|Lerp 0.0 1e+05 (Variables|Default|GetAccelerateInput)) (Variables|Default|GetAccelerateInput)))
  (Variables|Default|SetAccelerateInput (Math|Interpolation|FInterpTo (Variables|Default|GetAccelerateInput) 0.0 (Utilities|Time|GetWorldDeltaSeconds) 0.3)))

(fn Accelerate
  (params (WheelComp :type Scene%20Component%20Object%20Reference))
  (bind _box (Variables|Default|GetBox))
  (Class|PrimitiveComponent|AddForceatLocation (Variables|Default|GetBox) (* (Math|Vector|GetForwardVector _box) 1e+05 (Variables|Default|Getacceleration) (Physics|GetMass _box)) (Transformation|GetWorldLocation WheelComp) "None"))

(fn FOVDinamico
  (Camera|SetFieldOfView (Variables|Default|GetCamera) (Math|Float|Lerp (Variables|Default|GetFov%20quieto) (Variables|Default|GetFov%20Max) (Math|Float|Clamp(Float) (/ (Math|Vector|VectorLength (Transformation|GetVelocity)) (Variables|Default|GetVelocidad))))))